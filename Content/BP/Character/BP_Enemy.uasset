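; Enemy character Blueprint for a zombie-slaying game, handling player detection, death reporting and modular mesh setup.
; PawnSensing calls TrackingPlayer whenever it sees a pawn.
; DeadEnemySignal waits a few seconds, then passes the enemy's index to DieEnemy on ZombieSlayerGameMode.
; The construction script makes the extra skeletal mesh components follow the main Mesh through leader pose, so the body parts animate as one.
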(event `self.ReceiveBeginPlay`)

(event `self.PawnSensing.OnSeePawn`
  (params (Pawn :type "Pawn Object Reference"))
  (`self.TrackingPlayer`))

(event `self.DeadEnemySignal`
  (params (index :type Integer))
  (`KismetSystemLibrary.Delay` 3.0)
  (bind _aszombie_slayer_game_mode (cast `ZombieSlayerGameMode` (`GameplayStatics.GetGameMode`)))
  (`ZombieSlayerGameMode.DieEnemy` _aszombie_slayer_game_mode index))

(fn `UserConstructionScript`
  (`SkinnedMeshComponent.SetLeaderPoseComponent` (`self.SkeletalMesh7`) (`self.Mesh`) false false)
  (`SkinnedMeshComponent.SetLeaderPoseComponent` (`self.SkeletalMesh2`) (`self.Mesh`) false false)
  (`SkinnedMeshComponent.SetLeaderPoseComponent` (`self.SkeletalMesh3`) (`self.Mesh`) false false)
  (`SkinnedMeshComponent.SetLeaderPoseComponent` (`self.SkeletalMesh4`) (`self.Mesh`) false false)
  (`SkinnedMeshComponent.SetLeaderPoseComponent` (`self.SkeletalMesh5`) (`self.Mesh`) false false)
  (`SkinnedMeshComponent.SetLeaderPoseComponent` (`self.SkeletalMesh6`) (`self.Mesh`) false false)
  (`SkinnedMeshComponent.SetLeaderPoseComponent` (`self.SkeletalMesh7`) (`self.Mesh`) false false)
  (`SkinnedMeshComponent.SetLeaderPoseComponent` (`self.SkeletalMesh`) (`self.Mesh`) false false)
  (`SkinnedMeshComponent.SetLeaderPoseComponent` (`self.SkeletalMesh1`) (`self.Mesh`) false false)
  (`SkinnedMeshComponent.SetLeaderPoseComponent` (`self.SkeletalMesh8`) (`self.Mesh`) false false))